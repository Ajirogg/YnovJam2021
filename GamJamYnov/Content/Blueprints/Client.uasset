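; Client Blueprint that generates a random food order for the player to fulfil.
; TakeOrder builds a random row name from "Recipe" plus a random index and looks it up in the DT_Recipes data table.
; When the row is found, it prints the recipe's three ingredients on screen and flags the order as taken.
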(event `TakeOrder`
  (bind (_datatable _rowname) (break `DataTableRowHandle` (`self.Command`)))
  (bind _output_get (set `self.RandomRecipe` (`KismetStringLibrary.Conv_StringToName` (`KismetTextLibrary.Conv_TextToString` (`|FormatText` "Recipe{x}" (`KismetMathLibrary.RandomInteger` 5))))))
  (set `self.Command` (make `DataTableRowHandle` "/Game/Data/DT_Recipes.DT_Recipes" _output_get))
  (bind _returnvalue (`|GetDataTableRow` _datatable _rowname)
    (:`then`
      (bind (_recipemesh `_ingrédientn1` `_ingrédientn2` `_ingrédientn3`) (break `/Game/Data/ST_DT_Recipes` _returnvalue))
      (bind _output_get_2 (set `self.Needed` (`KismetTextLibrary.Conv_TextToString` (`|FormatText` "{1}   {2}   {3} " `_ingrédientn1` `_ingrédientn2` `_ingrédientn3`))))
      (`KismetSystemLibrary.PrintString` _output_get_2 true true (struct :`G` 0.66 :`B` 1.0 :`A` 1.0) 10.0)
      (set `self.IsOrderTaken` true))))

(fn `UserConstructionScript`)