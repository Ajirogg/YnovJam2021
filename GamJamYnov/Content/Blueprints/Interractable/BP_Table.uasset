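; BP_Table is an interactable table that spawns a customer and tracks their order through timed phases.
; SpawnCustomer starts a random delay, after which Tick spawns a client at AttachPoint and counts down its wait to order, then to be served.
; Timeouts report failure to GameManager and destroy the client.
; GiveOrder reports success with remaining time regardless of validity, which only changes a debug print.
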(event `SpawnCustomer`
  (params (MinTimerSpawn :type "Float (double-precision)") (MaxTimerSPawn :type "Float (double-precision)"))
  (set `self.MinRangeSpawn` MinTimerSpawn)
  (set `self.MaxRangeSpawn` MaxTimerSPawn)
  (set `self.Timer` (`KismetMathLibrary.RandomFloatInRange` (`self.MinRangeSpawn`) (`self.MaxRangeSpawn`)))
  (set `self.IsSpawning` true)
  (set `self.IsActive` true))

(event `self.ReceiveTick`
  (params (DeltaSeconds :type "Float (single-precision)"))
  (bind _attachpoint (`self.AttachPoint`))
  (if (`self.IsActive`)
    (bind _output_get (set `self.Timer` (- (`self.Timer`) DeltaSeconds)))
    (if (<= _output_get 0.0)
      (if (`self.IsSpawning`)
        (set `self.IsSpawning` false)
        (set `self.IsWaitingTakeOrder` true)
        (bind _returnvalue (`|SpawnActorFromClass` "/Game/Blueprints/Client.Client_C" (`KismetMathLibrary.MakeTransform` (`SceneComponent.K2_GetComponentLocation` _attachpoint) (`SceneComponent.K2_GetComponentRotation` _attachpoint)) "AlwaysSpawn" "OverrideRootScale" null null))
        (bind _output_get_2 (set `self.Client` _returnvalue))
        (`PrimitiveComponent.SetMaterial` (`/Game/Blueprints/Client.SkeletalMesh` _output_get_2) 0 "/Game/Art/Materials/M_Client_Bleu.M_Client_Bleu")
        (set `self.Timer` (`self.TimerTakeOrder`))
        (set `self.HadCustomer` true)
        (elif (`self.IsWaitingTakeOrder`)
          (`/Game/Blueprints/BP_Scoring.OrderNotTake` (`self.GameManager`) self)
          (set `self.IsActive` false)
          (`self.K2_DestroyActor` (`self.Client`))
          (set `self.IsWaitingTakeOrder` false)
          (set `self.HadCustomer` false)
          (elif (`self.IsWaitingHisOrder`)
            (`/Game/Blueprints/BP_Scoring.FailOrderCustomer` (`self.GameManager`) self)
            (set `self.IsActive` false)
            (`self.K2_DestroyActor` (`self.Client`))
            (set `self.IsWaitingHisOrder` false)
            (set `self.HadCustomer` false)))))))

(event `TakeCustomerOrder`
  (set `self.IsWaitingHisOrder` true)
  (set `self.IsWaitingTakeOrder` false)
  (set `self.Timer` (`self.TimerEndOrder `))
  (`/Game/Blueprints/Client.TakeOrder` (`self.Client`))
  (`KismetSystemLibrary.PrintString` "NEED TO BE LINK TO HUD"))

(event `GiveOrder`
  (params (IsValid :type Boolean))
  (if IsValid
    (`KismetSystemLibrary.PrintString` "Well Done")
    (else
      (`KismetSystemLibrary.PrintString` "F*ck you ")))
  (`self.K2_DestroyActor` (`self.Client`))
  (`/Game/Blueprints/BP_Scoring.OrderSuccess` (`self.GameManager`) self (`self.Timer`))
  (set `self.HadCustomer` false)
  (set `self.Timer` (`self.TimerTakeOrder`))
  (set `self.IsActive` false))

(fn `UserConstructionScript`
  (`parent.UserConstructionScript`))