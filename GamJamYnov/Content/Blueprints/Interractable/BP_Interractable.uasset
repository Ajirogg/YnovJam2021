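; BP_Interractable is a station for processing held objects such as ingredients, with trash and storage variants set by flags.
; StartUse destroys the object on trash; otherwise, non-storage stations snap it to AttachPoint and start a countdown.
; Tick runs the countdown, then a DoOnce marks the BP_Ingredient as transformed and swaps its mesh to a cone.
; StopUsing clears the state and object and resets the DoOnce.
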(event `StartUse`
  (if (`self.IsTrash`)
    (`self.K2_DestroyActor` (`self.Object`))
    (set `self.IsUsed` false)
    (elif (not (`self.IsStorage`))
      (`self.K2_SetActorLocation` (`self.Object`) (`SceneComponent.K2_GetComponentLocation` (`self.AttachPoint`)) false false)
      (set `self.timeUntilEnd` (`self.timeToFinished`))
      (set `self.IsUsed` true))))

(event `StopUsing`
  (set `self.IsUsed` false)
  (set `self.IsFinished` false)
  (set `self.Object` null)
  (goto _label :!via `Reset`))

(event `self.ReceiveTick`
  (params (DeltaSeconds :type "Float (single-precision)"))
  (if (`self.IsUsed`)
    (if (`self.IsFinished`)
      (`/Engine/EditorBlueprintResources/StandardMacros.DoOnce` false :!label _label
        (:`Completed`
          (if (not (`self.IsStorage`))
            (bind _asbp_ingredient (cast `/Game/Blueprints/Ingredients/BP_Ingredient` (`self.Object`)))
            (set `/Game/Blueprints/Ingredients/BP_Ingredient.IsTransformed` true _asbp_ingredient)
            (`StaticMeshComponent.SetStaticMesh` (`/Game/Blueprints/Ingredients/BP_Ingredient.StaticMesh` _asbp_ingredient) "/Engine/BasicShapes/Cone.Cone"))))
      (else
        (bind _output_get (set `self.timeUntilEnd` (- (`self.timeUntilEnd`) DeltaSeconds)))
        (if (<= _output_get 0.0)
          (set `self.IsFinished` true))))))

(fn `UserConstructionScript`)