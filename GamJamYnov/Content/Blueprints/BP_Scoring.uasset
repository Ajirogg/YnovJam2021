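; BP_Scoring manages customer flow and restaurant reputation, spawning customers at random BP_Table actors.
; BeginPlay gathers the tables and seats the first customer, then Tick requests more while the waiting count is below the maximum.
; Ignored or failed orders lower reputation, while successes raise it more when more time remains, and each outcome returns the table to the free pool.
; Reputation tiers set the maximum simultaneous customers, though some update paths skip clamping or tier recalculation.
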(event `self.ReceiveBeginPlay`
  (bind _outactors (`GameplayStatics.GetAllActorsOfClass` "/Game/Blueprints/Interractable/BP_Table.BP_Table_C"))
  (bind _output_get (set `self.Tables` _outactors))
  (set `self.TableWithoutCustomers` _output_get)
  (bind _output (`|GetArrayItem` _output_get (`KismetMathLibrary.RandomIntegerInRange` 0 (- (`KismetArrayLibrary.Array_Length` _output_get) 1))))
  (`/Game/Blueprints/Interractable/BP_Table.SpawnCustomer` _output (`self.MinWaitTimeBeforeNextCustom`) (`self.MaxWaitTimeBeforeNextCustom`))
  (`KismetArrayLibrary.Array_RemoveItem` (`self.TableWithoutCustomers`) _output)
  (`/Engine/EditorBlueprintResources/StandardMacros.IncrementInt` (`self.NbClientsWaiting`)))

(event `self.ReceiveTick`
  (params (DeltaSeconds :type "Float (single-precision)"))
  (bind _tablewithoutcustomers (`self.TableWithoutCustomers`))
  (bind _output (`|GetArrayItem` _tablewithoutcustomers (`KismetMathLibrary.RandomIntegerInRange` 0 (- (`KismetArrayLibrary.Array_Length` _tablewithoutcustomers) 1))))
  (if (> (`self.NbMaxClients`) (`self.NbClientsWaiting`))
    (`/Engine/EditorBlueprintResources/StandardMacros.IncrementInt` (`self.NbClientsWaiting`)
      (:`  `
        (`/Game/Blueprints/Interractable/BP_Table.SpawnCustomer` _output (`self.MinWaitTimeBeforeNextCustom`) (`self.MaxWaitTimeBeforeNextCustom`))
        (`KismetArrayLibrary.Array_RemoveItem` (`self.TableWithoutCustomers`) _output)))))

(event `OrderNotTake`
  (params (Table :type "/Game/Blueprints/Interractable/BP_Table Object Reference"))
  (bind _reputation (`self.Reputation`))
  (`/Engine/EditorBlueprintResources/StandardMacros.DecrementInt` (`self.NbClientsWaiting`)
    (:`  `
      (`KismetArrayLibrary.Array_Add` (`self.TableWithoutCustomers`) Table)
      (set `self.Reputation` (- (`self.Reputation`) 25.0))
      (if (<= _reputation 0.0) :!label _label
        (set `self.Reputation` 0.0)
        (if (< (`self.Reputation`) 16.5) :!label _label_2
          (set `self.NbMaxClients` 1)
          (elif (< (`self.Reputation`) 33.0)
            (set `self.NbMaxClients` 2)
            (elif (< (`self.Reputation`) 49.5)
              (set `self.NbMaxClients` 3)
              (elif (< (`self.Reputation`) 66.0)
                (set `self.NbMaxClients` 4)
                (elif (< (`self.Reputation`) 82.5)
                  (set `self.NbMaxClients` 5)
                  (else
                    (set `self.NbMaxClients` 6)))))))
        (elif (>= _reputation 99.0)
          (set `self.Reputation` 99.0)
          (goto _label_2))))))

(event `FailOrderCustomer`
  (params (Table :type "/Game/Blueprints/Interractable/BP_Table Object Reference"))
  (`/Engine/EditorBlueprintResources/StandardMacros.DecrementInt` (`self.NbClientsWaiting`)
    (:`  `
      (`KismetArrayLibrary.Array_Add` (`self.TableWithoutCustomers`) Table)
      (set `self.Reputation` (- (`self.Reputation`) 15.0))
      (goto _label))))

(event `OrderSuccess`
  (params (Table :type "/Game/Blueprints/Interractable/BP_Table Object Reference") (TimeRemain :type "Float (double-precision)"))
  (`/Engine/EditorBlueprintResources/StandardMacros.DecrementInt` (`self.NbClientsWaiting`)
    (:`  `
      (`KismetArrayLibrary.Array_Add` (`self.TableWithoutCustomers`) Table)
      (if (<= TimeRemain 15.0)
        (set `self.Reputation` (+ (`self.Reputation`) 10.0))
        (goto _label_2)
        (elif (<= TimeRemain 30.0)
          (set `self.Reputation` (+ (`self.Reputation`) 20.0))
          (goto _label_2)
          (else
            (set `self.Reputation` (+ (`self.Reputation`) 30.0))
            (goto _label_2)))))))

(fn `UserConstructionScript`)